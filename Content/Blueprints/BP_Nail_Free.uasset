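; A grabbable VR nail that is driven by BP_Hammer hits to fasten wooden plates together.
; While held by a motion controller near a nailing point, it locks to the plate's rotation each tick and can attach to that plate when hit.
; Further hits step it forward through Status stages, the last attaching an overlapping BP_WoodenPlateFree to the nail's parent.
; CanHit re-arms when the hammer leaves the capsule, preventing repeated hits.
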(event `self.HitBox.OnComponentHit`
  (params (HitComponent :type "PrimitiveComponent Object Reference") (OtherActor :type "Actor Object Reference") (OtherComp :type "PrimitiveComponent Object Reference") (NormalImpulse :type "Vector Structure") (Hit :type "HitResult Structure (by ref)"))
  (bind _item (`KismetArrayLibrary.Array_Get` (`PrimitiveComponent.GetOverlappingActors` (`self.Nail`) null) 1))
  (cast `/Game/Blueprints/BP_Hammer` OtherActor)
  (if (`self.CanHit`)
    (set `self.CanHit` false)
    (`KismetSystemLibrary.PrintString` "Hit")
    (if (== (`self.GetAttachParentActor`) null)
      (`self.AttachToPlate`)
      (else
        (`self.SetNailLocation`)
        (`KismetSystemLibrary.PrintString` (`KismetSystemLibrary.GetDisplayName` _item))
        (if (== (`self.Status`) -1)
          (bind _asbp_wooden_plate_free (cast `/Game/Blueprints/BP_WoodenPlateFree` _item)
            (:`then`
              (`/Game/Blueprints/BP_WoodenPlateFree.AttachToPlate` _asbp_wooden_plate_free (`self.GetAttachParentActor`)))
            (:`CastFailed`
              (`KismetSystemLibrary.PrintString` "fail"))))))))

(event `self.Capsule.OnComponentEndOverlap`
  (params (OverlappedComponent :type "PrimitiveComponent Object Reference") (OtherActor :type "Actor Object Reference") (OtherComp :type "PrimitiveComponent Object Reference") (OtherBodyIndex :type Integer))
  (cast `/Game/Blueprints/BP_Hammer` OtherActor)
  (set `self.CanHit` true))

(event `self.ReceiveTick`
  (params (DeltaSeconds :type "Float (single-precision)"))
  ;[1 1 1] 나무판에 닿았을때 못 방향 고정
  (if (`self.IsGrap`)
    (if (`self.IsNailingPoint`)
      (`self.K2_SetActorRotation` (`self.ClosedPlateRotator`)))))

(event `/Game/Character/I__GrabAble.Grab`
  (params (MotionCtrl :type "MotionControllerComponent Object Reference"))
  (`PrimitiveComponent.SetSimulatePhysics` (`self.Nail`) false)
  (`self.K2_AttachToComponent` MotionCtrl "None" "KeepWorld" "KeepWorld" "KeepWorld")
  (set `self.IsGrap` true))

(event `/Game/Character/I__GrabAble.Release`
  (`PrimitiveComponent.SetSimulatePhysics` (`self.Nail`) true)
  (`self.K2_DetachFromActor` "KeepWorld" "KeepWorld" "KeepWorld")
  (set `self.IsGrap` false))

(fn `AttachToPlate`
  (bind _closedplateofnailingpoint (`self.ClosedPlateOfNailingPoint`))
  (if (`self.IsNailingPoint`)
    (if (!= _closedplateofnailingpoint null)
      (`self.K2_AttachToActor` _closedplateofnailingpoint "None" "KeepWorld" "KeepWorld" "KeepWorld")
      (`KismetSystemLibrary.PrintString` "붙음")
      (`PrimitiveComponent.SetCollisionObjectType` (`self.Capsule`) "ECC_GameTraceChannel3")
      (`PrimitiveComponent.SetCollisionObjectType` (`self.Nail`) "ECC_GameTraceChannel3")
      (set `self.IsGrap` false))))

(fn `SetNailLocation`
  (locals (Value :type "Float (double-precision)"))
  (bind _status (`self.Status`))
  (bind _direction (`self.Direction`))
  (if (== _status 2)
    (set `local.Value` 8.0)
    (`self.K2_SetActorLocation` (+ (`SceneComponent.GetSocketLocation` _direction "None") (* (`KismetMathLibrary.GetForwardVector` (`SceneComponent.GetSocketRotation` _direction "None")) (`local.Value`))) :!label _label)
    (set `self.Status` (- (`self.Status`) 1))
    (elif (== _status 1)
      (set `local.Value` 7.0)
      (goto _label)
      (elif (== _status 0)
        (set `local.Value` 7.0)
        (goto _label)))))

(fn `UserConstructionScript`)