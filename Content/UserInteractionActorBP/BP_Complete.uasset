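; BP_Complete is an assembly guide actor with five long and two short wooden plate slots that detect matching free plates brought near them.
; Overlap handlers ignore plates attached to BP_Origin, recolour a close slot through a dynamic M_MakerGuide material, and store it as the plate's ClosedGuide.
; OverlappedGuide tracks the highlighted slot; leaving it clears both references and restores the colour.
; SetPlateToGuide resets the colour and OverlappedGuide, without moving the plate.
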(event `self.SM_WoodenPlate.OnComponentBeginOverlap`
  (params (OverlappedComponent :type "PrimitiveComponent Object Reference") (OtherActor :type "Actor Object Reference") (OtherComp :type "PrimitiveComponent Object Reference") (OtherBodyIndex :type Integer) (bFromSweep :type Boolean) (SweepResult :type "HitResult Structure (by ref)"))
  (`self.BeginOverlapPlate` OverlappedComponent OtherActor))

(event `self.SM_WoodenPlate2.OnComponentBeginOverlap`
  (params (OverlappedComponent :type "PrimitiveComponent Object Reference") (OtherActor :type "Actor Object Reference") (OtherComp :type "PrimitiveComponent Object Reference") (OtherBodyIndex :type Integer) (bFromSweep :type Boolean) (SweepResult :type "HitResult Structure (by ref)"))
  (`self.BeginOverlapPlate` OverlappedComponent OtherActor))

(event `self.SM_WoodenPlate3.OnComponentBeginOverlap`
  (params (OverlappedComponent :type "PrimitiveComponent Object Reference") (OtherActor :type "Actor Object Reference") (OtherComp :type "PrimitiveComponent Object Reference") (OtherBodyIndex :type Integer) (bFromSweep :type Boolean) (SweepResult :type "HitResult Structure (by ref)"))
  (`self.BeginOverlapPlate` OverlappedComponent OtherActor))

(event `self.SM_WoodenPlate4.OnComponentBeginOverlap`
  (params (OverlappedComponent :type "PrimitiveComponent Object Reference") (OtherActor :type "Actor Object Reference") (OtherComp :type "PrimitiveComponent Object Reference") (OtherBodyIndex :type Integer) (bFromSweep :type Boolean) (SweepResult :type "HitResult Structure (by ref)"))
  (`self.BeginOverlapPlate` OverlappedComponent OtherActor))

(event `self.SM_WoodenPlate5.OnComponentBeginOverlap`
  (params (OverlappedComponent :type "PrimitiveComponent Object Reference") (OtherActor :type "Actor Object Reference") (OtherComp :type "PrimitiveComponent Object Reference") (OtherBodyIndex :type Integer) (bFromSweep :type Boolean) (SweepResult :type "HitResult Structure (by ref)"))
  (`self.BeginOverlapPlate` OverlappedComponent OtherActor))

(event `self.SM_ShortWoodenPlate.OnComponentBeginOverlap`
  (params (OverlappedComponent :type "PrimitiveComponent Object Reference") (OtherActor :type "Actor Object Reference") (OtherComp :type "PrimitiveComponent Object Reference") (OtherBodyIndex :type Integer) (bFromSweep :type Boolean) (SweepResult :type "HitResult Structure (by ref)"))
  (`self.BeginOverlapShortPlate` OverlappedComponent OtherActor))

(event `self.SM_ShortWoodenPlate2.OnComponentBeginOverlap`
  (params (OverlappedComponent :type "PrimitiveComponent Object Reference") (OtherActor :type "Actor Object Reference") (OtherComp :type "PrimitiveComponent Object Reference") (OtherBodyIndex :type Integer) (bFromSweep :type Boolean) (SweepResult :type "HitResult Structure (by ref)"))
  (`self.BeginOverlapShortPlate` OverlappedComponent OtherActor))

(event `self.SM_WoodenPlate.OnComponentEndOverlap`
  (params (OverlappedComponent :type "PrimitiveComponent Object Reference") (OtherActor :type "Actor Object Reference") (OtherComp :type "PrimitiveComponent Object Reference") (OtherBodyIndex :type Integer))
  (`self.EndOverlapPlate` OverlappedComponent OtherActor))

(event `self.SM_WoodenPlate2.OnComponentEndOverlap`
  (params (OverlappedComponent :type "PrimitiveComponent Object Reference") (OtherActor :type "Actor Object Reference") (OtherComp :type "PrimitiveComponent Object Reference") (OtherBodyIndex :type Integer))
  (`self.EndOverlapPlate` OverlappedComponent OtherActor))

(event `self.SM_WoodenPlate3.OnComponentEndOverlap`
  (params (OverlappedComponent :type "PrimitiveComponent Object Reference") (OtherActor :type "Actor Object Reference") (OtherComp :type "PrimitiveComponent Object Reference") (OtherBodyIndex :type Integer))
  (`self.EndOverlapPlate` OverlappedComponent OtherActor))

(event `self.SM_WoodenPlate4.OnComponentEndOverlap`
  (params (OverlappedComponent :type "PrimitiveComponent Object Reference") (OtherActor :type "Actor Object Reference") (OtherComp :type "PrimitiveComponent Object Reference") (OtherBodyIndex :type Integer))
  (`self.EndOverlapPlate` OverlappedComponent OtherActor))

(event `self.SM_WoodenPlate5.OnComponentEndOverlap`
  (params (OverlappedComponent :type "PrimitiveComponent Object Reference") (OtherActor :type "Actor Object Reference") (OtherComp :type "PrimitiveComponent Object Reference") (OtherBodyIndex :type Integer))
  (`self.EndOverlapPlate` OverlappedComponent OtherActor))

(event `self.SM_ShortWoodenPlate.OnComponentEndOverlap`
  (params (OverlappedComponent :type "PrimitiveComponent Object Reference") (OtherActor :type "Actor Object Reference") (OtherComp :type "PrimitiveComponent Object Reference") (OtherBodyIndex :type Integer))
  (`self.EndOverlapShortPlate` OverlappedComponent OtherActor))

(event `self.SM_ShortWoodenPlate2.OnComponentEndOverlap`
  (params (OverlappedComponent :type "PrimitiveComponent Object Reference") (OtherActor :type "Actor Object Reference") (OtherComp :type "PrimitiveComponent Object Reference") (OtherBodyIndex :type Integer))
  (`self.EndOverlapShortPlate` OverlappedComponent OtherActor))

(fn `BeginOverlapPlate`
  (params (OverlappedComponent :type "PrimitiveComponent Object Reference") (ClosedActor :type "Actor Object Reference"))
  (if (== (`self.Overlapped Guide`) null)
    (bind _asbp_wooden_plate_free (cast `/Game/UserInteractionActorBP/BP_WoodenPlateFree` ClosedActor))
    (cast `/Game/UserInteractionActorBP/BP_WoodenPlateFree_Short` ClosedActor
      (:`CastFailed`
        (cast `/Game/UserInteractionActorBP/BP_Origin` (`self.GetAttachParentActor` ClosedActor)
          (:`CastFailed`
            (if (< (`KismetMathLibrary.VSize` (- (`SceneComponent.K2_GetComponentLocation` OverlappedComponent) (`self.K2_GetActorLocation` ClosedActor))) 100.0)
              (bind _returnvalue (`PrimitiveComponent.CreateDynamicMaterialInstance` OverlappedComponent 0 "/Game/Materials/M_MakerGuide.M_MakerGuide"))
              (bind _output_get (set `self.Overlapped Mat` _returnvalue))
              (`MaterialInstanceDynamic.SetVectorParameterValue` _output_get "Color" (struct :`R` 0.6 :`G` 0.146455 :`B` 0.23663 :`A` 1.0))
              (bind _output_get_2 (set `self.Overlapped Guide` OverlappedComponent))
              (set `/Game/UserInteractionActorBP/BP_WoodenPlateFree.ClosedGuide` _output_get_2 _asbp_wooden_plate_free))))))))

(fn `BeginOverlapShortPlate`
  (params (OverlappedComponent :type "PrimitiveComponent Object Reference") (ClosedActor :type "Actor Object Reference"))
  (if (== (`self.Overlapped Guide`) null)
    (bind _asbp_wooden_plate_free_short (cast `/Game/UserInteractionActorBP/BP_WoodenPlateFree_Short` ClosedActor))
    (cast `/Game/UserInteractionActorBP/BP_Origin` (`self.GetAttachParentActor` ClosedActor)
      (:`CastFailed`
        (if (< (`KismetMathLibrary.VSize` (- (`SceneComponent.K2_GetComponentLocation` OverlappedComponent) (`self.K2_GetActorLocation` ClosedActor))) 100.0)
          (bind _returnvalue (`PrimitiveComponent.CreateDynamicMaterialInstance` OverlappedComponent 0 "/Game/Materials/M_MakerGuide.M_MakerGuide"))
          (bind _output_get (set `self.Overlapped Mat` _returnvalue))
          (`MaterialInstanceDynamic.SetVectorParameterValue` _output_get "Color" (struct :`R` 0.6 :`G` 0.146455 :`B` 0.23663 :`A` 1.0))
          (bind _output_get_2 (set `self.Overlapped Guide` OverlappedComponent))
          (set `/Game/UserInteractionActorBP/BP_WoodenPlateFree.ClosedGuide` _output_get_2 _asbp_wooden_plate_free_short))))))

(fn `EndOverlapPlate`
  (params (OverlappedComponent :type "PrimitiveComponent Object Reference") (ClosedActor :type "Actor Object Reference"))
  (bind _asbp_wooden_plate_free (cast `/Game/UserInteractionActorBP/BP_WoodenPlateFree` ClosedActor))
  (if (== (`self.Overlapped Guide`) OverlappedComponent)
    (cast `/Game/UserInteractionActorBP/BP_WoodenPlateFree_Short` ClosedActor
      (:`CastFailed`
        (cast `/Game/UserInteractionActorBP/BP_Origin` (`self.GetAttachParentActor` ClosedActor)
          (:`CastFailed`
            (`MaterialInstanceDynamic.SetVectorParameterValue` (`self.Overlapped Mat`) "Color" (struct :`R` 0.13 :`G` 1.0 :`B` 0.978 :`A` 1.0))
            (set `self.Overlapped Guide` null)
            (set `/Game/UserInteractionActorBP/BP_WoodenPlateFree.ClosedGuide` null _asbp_wooden_plate_free)))))))

(fn `EndOverlapShortPlate`
  (params (OverlappedComponent :type "PrimitiveComponent Object Reference") (ClosedActor :type "Actor Object Reference"))
  (bind _asbp_wooden_plate_free_short (cast `/Game/UserInteractionActorBP/BP_WoodenPlateFree_Short` ClosedActor))
  (if (== (`self.Overlapped Guide`) OverlappedComponent)
    (cast `/Game/UserInteractionActorBP/BP_Origin` (`self.GetAttachParentActor` ClosedActor)
      (:`CastFailed`
        (`MaterialInstanceDynamic.SetVectorParameterValue` (`self.Overlapped Mat`) "Color" (struct :`R` 0.13 :`G` 1.0 :`B` 0.978 :`A` 1.0))
        (set `self.Overlapped Guide` null)
        (set `/Game/UserInteractionActorBP/BP_WoodenPlateFree.ClosedGuide` null _asbp_wooden_plate_free_short)))))

(fn `SetPlateToGuide`
  (`MaterialInstanceDynamic.SetVectorParameterValue` (`self.Overlapped Mat`) "Color" (struct :`R` 0.13 :`G` 1.0 :`B` 0.978 :`A` 1.0))
  (set `self.Overlapped Guide` null))

(fn `UserConstructionScript`)