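; Grabbable wooden plate that can be joined to other plates with nails or placed onto a build guide.
; Two nailing-point overlaps give entering BP_Nail_Free actors their rotation and plate reference, clearing the point on exit.
; AttachToPlate groups plates through attachment, spawning a shared BP_Origin for an unattached pair, so Grab moves the parent.
; On release, a lone plate near a guide hands off to BP_Complete_Attach and destroys itself.
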(event `self.NailingUpPoint.OnComponentBeginOverlap`
  (params (OverlappedComponent :type "PrimitiveComponent Object Reference") (OtherActor :type "Actor Object Reference") (OtherComp :type "PrimitiveComponent Object Reference") (OtherBodyIndex :type Integer) (bFromSweep :type Boolean) (SweepResult :type "HitResult Structure (by ref)"))
  ;[1 1 1] 못이 Collision안에 있으면 못의 방향 고정
  (set `self.NailPointRotator` (`SceneComponent.K2_GetComponentRotation` (`self.NailingUpPoint`)))
  (`self.SendBoxRotatorToNail` OtherActor))

(event `self.NailingDownPoint.OnComponentBeginOverlap`
  (params (OverlappedComponent :type "PrimitiveComponent Object Reference") (OtherActor :type "Actor Object Reference") (OtherComp :type "PrimitiveComponent Object Reference") (OtherBodyIndex :type Integer) (bFromSweep :type Boolean) (SweepResult :type "HitResult Structure (by ref)"))
  ;[1 1 1] 못이 Collision안에 있으면 못의 방향 고정
  (set `self.NailPointRotator` (`SceneComponent.K2_GetComponentRotation` (`self.NailingDownPoint`)))
  (`self.SendBoxRotatorToNail` OtherActor))

(event `self.NailingUpPoint.OnComponentEndOverlap`
  (params (OverlappedComponent :type "PrimitiveComponent Object Reference") (OtherActor :type "Actor Object Reference") (OtherComp :type "PrimitiveComponent Object Reference") (OtherBodyIndex :type Integer))
  ;[1 1 1] Collision에서 나가면 못의 위치 방향 고정 해제
  (bind _asbp_nail_free (cast `/Game/UserInteractionActorBP/BP_Nail_Free` OtherActor))
  (set `/Game/UserInteractionActorBP/BP_Nail_Free.IsNailingPoint` false _asbp_nail_free)
  (set `/Game/UserInteractionActorBP/BP_Nail_Free.ClosedPlateOfNailingPoint` null _asbp_nail_free))

(event `self.NailingDownPoint.OnComponentEndOverlap`
  (params (OverlappedComponent :type "PrimitiveComponent Object Reference") (OtherActor :type "Actor Object Reference") (OtherComp :type "PrimitiveComponent Object Reference") (OtherBodyIndex :type Integer))
  ;[1 1 1] Collision에서 나가면 못의 위치 방향 고정 해제
  (bind _asbp_nail_free (cast `/Game/UserInteractionActorBP/BP_Nail_Free` OtherActor))
  (set `/Game/UserInteractionActorBP/BP_Nail_Free.IsNailingPoint` false _asbp_nail_free)
  (set `/Game/UserInteractionActorBP/BP_Nail_Free.ClosedPlateOfNailingPoint` null _asbp_nail_free))

(event `/Game/Character/I__GrabAble.Release`
  (bind _returnvalue (`self.GetAttachParentActor`))
  (bind _closedguide (`self.ClosedGuide`))
  (cast `/Game/UserInteractionActorBP/BP_Origin` _returnvalue
    (:`then`
      (`self.K2_DetachFromActor` _returnvalue "KeepWorld" "KeepWorld" "KeepWorld"))
    (:`CastFailed`
      (`self.K2_DetachFromActor` "KeepWorld" "KeepWorld" "KeepWorld")
      (if (!= _closedguide null)
        (`self.K2_SetActorTransform` (`SceneComponent.K2_GetComponentToWorld` _closedguide))
        (bind _asbp_complete_attach (cast `/Game/UserInteractionActorBP/BP_Complete_Attach` (`ActorComponent.GetOwner` _closedguide)))
        (`/Game/UserInteractionActorBP/BP_Complete_Attach.SetPlateToGuide` _asbp_complete_attach _closedguide)
        (set `self.ClosedGuide` null)
        (`self.K2_DestroyActor`)))))

(fn `AttachToPlate`
  (params (PlateOfAttachedNail :type "Actor Object Reference"))
  (locals (PlateOfAttachedNail_Local :type "/Game/UserInteractionActorBP/BP_WoodenPlateFree Object Reference"))
  (bind _returnvalue (`self.GetAttachParentActor`))
  (bind _returnvalue_2 (`self.GetAttachParentActor`))
  (bind _plateofattachednail_local (`local.PlateOfAttachedNail_Local`))
  (bind _asbp_wooden_plate_free (cast `/Game/UserInteractionActorBP/BP_WoodenPlateFree` PlateOfAttachedNail))
  (set `local.PlateOfAttachedNail_Local` _asbp_wooden_plate_free)
  (if (!= (`self.GetAttachParentActor` _asbp_wooden_plate_free) null)
    (if (!= _returnvalue_2 null)
      (`self.K2_AttachToActor` _returnvalue_2 (`self.GetAttachParentActor` _plateofattachednail_local) "None" "KeepWorld" "KeepWorld" "KeepWorld" true) ; 둘다 BP_Origin을 가지고 있으면 BP_origin에 BP_origin을 붙임.
      (else
        (`self.K2_AttachToActor` _plateofattachednail_local "None" "KeepWorld" "KeepWorld" "KeepWorld") ; 못이 박혀있는 Plate에 Origin이 있고 This.Plate에는 Origin이 없으면 존재하는 Origin에 붙임
      ))
    (elif (!= _returnvalue null)
      (`self.K2_AttachToActor` (`local.PlateOfAttachedNail_Local`) _returnvalue "None" "KeepWorld" "KeepWorld" "KeepWorld" true)
      (else
        ;[1 1 1] 처음 두개를 붙일 때 오리진 생성 후 둘다 붙임
        (bind _returnvalue_3 (`|SpawnActorFromClass` "/Game/UserInteractionActorBP/BP_Origin.BP_Origin_C" (`self.GetTransform`) "Undefined" "OverrideRootScale"))
        (`self.K2_AttachToActor` _returnvalue_3 "None" "KeepWorld" "KeepWorld" "KeepWorld")
        (`self.K2_AttachToActor` (`local.PlateOfAttachedNail_Local`) _returnvalue_3 "None" "KeepWorld" "KeepWorld" "KeepWorld" true)))))

(fn `Grab`
  (params (MotionCtrl :type "MotionControllerComponent Object Reference"))
  (returns (Actor :type "Actor Object Reference"))
  (bind _returnvalue (`self.GetAttachParentActor`))
  (if (== _returnvalue null)
    (`self.K2_AttachToComponent` MotionCtrl "None" "KeepWorld" "KeepWorld" "KeepWorld")
    (return self)
    (else
      (`self.K2_AttachToComponent` _returnvalue MotionCtrl "None" "KeepWorld" "KeepWorld" "KeepWorld" true)
      (return _returnvalue))))

(fn `SendBoxRotatorToNail`
  (params (`Other Actor` :type "Actor Object Reference"))
  (bind _asbp_nail_free (cast `/Game/UserInteractionActorBP/BP_Nail_Free` `Other Actor`))
  (set `/Game/UserInteractionActorBP/BP_Nail_Free.IsNailingPoint` true _asbp_nail_free)
  (set `/Game/UserInteractionActorBP/BP_Nail_Free.ClosedPlateRotator` (`self.NailPointRotator`) _asbp_nail_free)
  (set `/Game/UserInteractionActorBP/BP_Nail_Free.ClosedPlateOfNailingPoint` self _asbp_nail_free)
  (`KismetSystemLibrary.PrintString` "set Nailpoint"))

(fn `UserConstructionScript`)