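; BP_CarpenterMode is a game mode that handles the start sequence for the Carpenter mode.
; Tick polls for a left motion controller shoulder press until IsStart is set.
; The press creates a UI_FadeOut widget and drives its opacity with a FadeOut timeline.
; When that finishes, it moves the player character to the player start, destroys the StartWidget actor and runs FadeIn on the same widget.
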(event `self.ReceiveTick`
  (params (DeltaSeconds :type "Float (single-precision)"))
  (bind _returnvalue (`GameplayStatics.GetPlayerController` 0))
  (if (`self.is start`)
    _
    (elif (`PlayerController.WasInputKeyJustPressed` (`GameplayStatics.GetPlayerController` 0) "MotionController_Left_Shoulder")
      (set `self.is start` true)
      (bind _returnvalue_2 (`|CreateWidget` "/Game/Widget/UI_FadeOut.UI_FadeOut_C" _returnvalue))
      (`UserWidget.AddToViewport` _returnvalue_2 0)
      (bind (_direction _newtrack_1) (`Timeline|FadeOut`)
        (:`Update`
          (bind _fadeout (`/Game/Widget/UI_FadeOut.FadeOut` _returnvalue_2))
          (`Image.SetOpacity` _fadeout _newtrack_1))
        (:`Finished`
          (`self.K2_SetActorTransform` (`GameplayStatics.GetPlayerCharacter` 0) (`self.GetTransform` (`self.K2_FindPlayerStart` _returnvalue)) false false)
          (`self.K2_DestroyActor` (`self.StartWidget`))
          (bind (_direction_2 _newtrack_3) (`Timeline|FadeIn`)
            (:`Update`
              (`Image.SetOpacity` _fadeout _newtrack_3))))))))

(fn `UserConstructionScript`)