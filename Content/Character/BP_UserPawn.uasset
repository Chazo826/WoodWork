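; VR player pawn with motion-controller teleporting, object grabbing and mouse-look for testing.
; Holding TeleportR predicts a projectile arc each tick, drawn with spline meshes on near-flat surfaces; release moves Scene to the stored point if CanTeleport is set.
; Grab inputs toggle one shared held actor, found among hand-sphere overlaps through the I__GrabAble interface.
; A right face button spawns BP_Hammer straight into the right hand.
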(event `self.ReceiveTick`
  (params (DeltaSeconds :type "Float (single-precision)"))
  (bind _r_motioncontroller (`self.R_MotionController`))
  (if (`self.FindTeleport`)
    (`self.ClearSpline`)
    (`self.LocationDetect` (`SceneComponent.K2_GetComponentLocation` _r_motioncontroller) (`SceneComponent.GetForwardVector` _r_motioncontroller))))

(event `InputAction|TeleportR`
  (params (Key :type "Key Structure" :default "AnyKey"))
  (:`Pressed`
    (set `self.FindTeleport` true))
  (:`Released`
    (set `self.FindTeleport` false)
    (`self.ClearSpline`)
    (if (`self.CanTeleport`)
      (`SceneComponent.K2_SetWorldLocation` (`self.Scene`) (`KismetMathLibrary.MakeVector` (.x (`self.TeleLocation`)) (.y (`self.TeleLocation`)) (+ (.z (`self.TeleLocation`)) 100.0)) false false))))

(event `InputAxis|Turn`
  (params (AxisValue :type "Float (single-precision)"))
  ;[1 1 1] 마우스 테스트
  (`SceneComponent.K2_AddRelativeRotation` (`self.Camera`) (`KismetMathLibrary.MakeRotator` 0.0 0.0 AxisValue) false false))

(event `InputAxis|LookUp`
  (params (AxisValue :type "Float (single-precision)"))
  ;[1 1 1] 마우스 테스트
  (`SceneComponent.K2_AddRelativeRotation` (`self.Camera`) (* (`KismetMathLibrary.MakeRotator` 0.0 AxisValue) -1) false false))

(event `Key|MotionController_Right_Thumbstick_Left`
  (params (Key :type "Key Structure" :default "AnyKey"))
  (:`Pressed`
    (`KismetSystemLibrary.PrintString` "Thumbstick Left")))

(event `Key|MotionController_Right_FaceButton1`
  (params (Key :type "Key Structure" :default "AnyKey"))
  (:`Pressed`
    (if (not (`self.IsHammer`))
      (bind _returnvalue (`|SpawnActorFromClass` "/Game/UserInteractionActorBP/BP_Hammer.BP_Hammer_C" (`SceneComponent.K2_GetComponentToWorld` (`self.R_MotionController`)) "Undefined" "OverrideRootScale"))
      (set `self.IsGrabbleAct` true)
      (bind _actor (message `/Game/Character/I__GrabAble.Grab` _returnvalue (`self.R_MotionController`)))
      (set `self.AttachedActor` _actor))))

(event `InputAction|GrabL`
  (params (Key :type "Key Structure" :default "AnyKey"))
  (bind _l_motioncontroller (`self.L_MotionController`))
  ;[1 1 1] 그랩
  (:`Pressed`
    (if (`self.IsGrabbleAct`)
      (`self.ReleaseFunc` _l_motioncontroller)
      (else
        (`self.GrabFunc` (`self.L_Sphere`) _l_motioncontroller)))))

(event `InputAction|GrabR`
  (params (Key :type "Key Structure" :default "AnyKey"))
  (bind _r_motioncontroller (`self.R_MotionController`))
  ;[1 1 1] 그랩
  (:`Pressed`
    (if (`self.IsGrabbleAct`)
      (`self.ReleaseFunc` _r_motioncontroller)
      (else
        (`self.GrabFunc` (`self.R_Sphere`) _r_motioncontroller)))))

(fn `ClearSpline`
  (bind _splinemeshs (`self.SplineMeshs`))
  (`ActorComponent.K2_DestroyComponent` _splinemeshs)
  (`KismetArrayLibrary.Array_Clear` _splinemeshs)
  (`SplineComponent.ClearSplinePoints` (`self.Spline`) true))

(fn `Grab`
  (params (MotionCtrl :type "MotionControllerComponent Object Reference"))
  (returns (Actor :type "Actor Object Reference"))
  (return null))

(fn `GrabFunc`
  (params (Sphere :type "SphereComponent Object Reference") (MotionController :type "MotionControllerComponent Object Reference"))
  (bind _nearactor (`self.IsNearGrabFunc` Sphere))
  (`/Engine/EditorBlueprintResources/StandardMacros.IsValid` _nearactor
    (:`Is Valid`
      (set `self.IsGrabbleAct` true)
      (bind _actor (message `/Game/Character/I__GrabAble.Grab` _nearactor MotionController))
      (set `self.AttachedActor` _actor))))

(fn `IsNearGrabFunc`
  (params (Sphere :type "SphereComponent Object Reference"))
  (returns (NearActor :type "Actor Object Reference"))
  (for _array_element (`PrimitiveComponent.GetOverlappingActors` Sphere null)
    (if (`KismetSystemLibrary.DoesImplementInterface` _array_element "/Game/Character/I__GrabAble.I__GrabAble_C")
      (if (< (`KismetMathLibrary.VSize` (- (`self.K2_GetActorLocation` _array_element) (`SceneComponent.K2_GetComponentLocation` (`self.L_Sphere`)))) 300.0)
        (set `self.NearActor` _array_element))))
  (return (`self.NearActor`)))

(fn `LocationDetect`
  (params (CtrlLocation :type "Vector Structure") (CtrlForward :type "Vector Structure"))
  (bind (_outhit _outpathpositions) (`GameplayStatics.Blueprint_PredictProjectilePath_ByObjectType` CtrlLocation (* CtrlForward 1000.0) true 0.0 (`|MakeArray` "ObjectTypeQuery1" :!type "EObjectTypeQuery Enum") true)) ; 곡선(투사체의 궤적을 미리 그려주는 얘)
  (bind (_bblockinghit _binitialoverlap _time _location _impactpoint _normal) (`GameplayStatics.BreakHitResult` _outhit))
  (bind _returnvalue (> (`KismetMathLibrary.Dot_VectorVector` _normal (0.0 0.0 1.0)) 0.7))
  (if _returnvalue
    (bind _output_get (set `self.CanTeleport` _returnvalue))
    (`self.SplineUpdate` _output_get _outpathpositions)
    (set `self.TeleLocation` _location)))

(fn `ReleaseFunc`
  (params (MotionController :type "MotionControllerComponent Object Reference"))
  (bind _attachedactor (`self.AttachedActor`))
  (`/Engine/EditorBlueprintResources/StandardMacros.IsValid` _attachedactor
    (:`Is Valid`
      (if (== (`SceneComponent.GetAttachParent` (`self.K2_GetRootComponent` _attachedactor)) MotionController)
        (message `/Game/Character/I__GrabAble.Release` (`self.AttachedActor`)))
      (set `self.AttachedActor` null)
      (set `self.IsGrabbleAct` false)
      (set `self.NearActor` null))))

(fn `SplineUpdate`
  (params (canTeleport :type Boolean) (LocationVectors :type "Array of Vector Structure"))
  (bind _spline (`self.Spline`))
  (bind _spline_2 (`self.Spline`))
  (bind _spline_3 (`self.Spline`))
  (bind _returnvalue (`SceneComponent.K2_GetComponentLocation` _spline_3))
  (if canTeleport
    (for _array_element LocationVectors
      (`SplineComponent.AddSplinePoint` _spline _array_element "Local" true))
    (`SplineComponent.SetSplinePointType` _spline (`KismetArrayLibrary.Array_LastIndex` LocationVectors) "CurveClamped" true)
    (for _index (range (+ (- (`SplineComponent.GetNumberOfSplinePoints` (`self.Spline`)) 2) 1))
      (bind _returnvalue_2 (`AddComponent|NODE_AddSplineMeshComponent-0` :`bManualAttachment` true :`RelativeTransform` (`KismetMathLibrary.MakeTransform` (0.0 0.0 0.0) (struct) (1.0 1.0 1.0))))
      (`KismetArrayLibrary.Array_Add` (`self.SplineMeshs`) _returnvalue_2)
      (bind _returnvalue_3 (+ _index 1))
      (`SplineMeshComponent.SetStartAndEnd` _returnvalue_2 (`KismetArrayLibrary.Array_Get` LocationVectors _index) (`SplineComponent.GetTangentAtSplinePoint` _spline_2 _index "Local") (`KismetArrayLibrary.Array_Get` LocationVectors _returnvalue_3) (`SplineComponent.GetTangentAtSplinePoint` _spline_2 _returnvalue_3 "Local") true))
    (else
      (`KismetArrayLibrary.Array_Clear` LocationVectors)
      (`KismetArrayLibrary.Array_Add` LocationVectors _returnvalue)
      (`KismetArrayLibrary.Array_Add` LocationVectors (+ _returnvalue (* (`SceneComponent.GetForwardVector` _spline_3) 20))))))

(fn `UserConstructionScript`)