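; BP_TestPawn is a test pawn with mouse-driven camera look, free movement along three axes and left-hand grabbing.
; GrabL toggles between grab and release, searching the hand sphere's overlaps for an I__GrabAble actor within range.
; Grab and release go through interface messages with the motion controller, caching the held actor and flagging a BP_Hammer.
; Left-sphere overlaps print actor names for debugging.
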(event `InputAxis|Turn`
  (params (AxisValue :type "Float (single-precision)"))
  ;[1 1 1] 마우스 테스트
  (`SceneComponent.K2_AddRelativeRotation` (`self.Camera`) (`KismetMathLibrary.MakeRotator` 0.0 0.0 AxisValue) false false))

(event `InputAxis|LookUp`
  (params (AxisValue :type "Float (single-precision)"))
  ;[1 1 1] 마우스 테스트
  (`SceneComponent.K2_AddRelativeRotation` (`self.Camera`) (`KismetMathLibrary.MakeRotator` 0.0 AxisValue) false false))

(event `InputAction|GrabL`
  (params (Key :type "Key Structure" :default "AnyKey"))
  (bind _motioncontroller (`self.MotionController`))
  ;[1 1 1] 그랩
  (:`Pressed`
    (if (`self.IsGrabbleAct`)
      (`self.ReleaseFunc` _motioncontroller)
      (else
        (`self.GrabFunc` (`self.L_Sphere`) _motioncontroller)))))

(event `InputAxis|InputForward`
  (params (AxisValue :type "Float (single-precision)"))
  (`self.K2_SetActorLocation` (+ (`self.K2_GetActorLocation`) (* (`KismetMathLibrary.GetForwardVector` (`KismetMathLibrary.MakeRotator` 0.0 0.0 (.yaw (`self.GetControlRotation`)))) (* (`self.Movement`) AxisValue)))))

(event `InputAxis|InputRight`
  (params (AxisValue :type "Float (single-precision)"))
  (`self.K2_SetActorLocation` (+ (* (`KismetMathLibrary.GetRightVector` (`KismetMathLibrary.MakeRotator` 0.0 0.0 (.yaw (`self.GetControlRotation`)))) (* (`self.Movement`) AxisValue)) (`self.K2_GetActorLocation`))))

(event `InputAxis|InputUp`
  (params (AxisValue :type "Float (single-precision)"))
  (`self.K2_SetActorLocation` (+ (`self.K2_GetActorLocation`) (* (`KismetMathLibrary.MakeVector` 0.0 0.0 (`KismetMathLibrary.Conv_IntToDouble` (`self.Movement`))) AxisValue))))

(event `self.L_Sphere.OnComponentBeginOverlap`
  (params (OverlappedComponent :type "PrimitiveComponent Object Reference") (OtherActor :type "Actor Object Reference") (OtherComp :type "PrimitiveComponent Object Reference") (OtherBodyIndex :type Integer) (bFromSweep :type Boolean) (SweepResult :type "HitResult Structure (by ref)"))
  (`KismetSystemLibrary.PrintString` (`KismetSystemLibrary.GetDisplayName` OtherActor)))

(fn `Grab`
  (params (MotionCtrl :type "MotionControllerComponent Object Reference"))
  (returns (Actor :type "Actor Object Reference"))
  (return null))

(fn `GrabFunc`
  (params (Sphere :type "SphereComponent Object Reference") (MotionController :type "MotionControllerComponent Object Reference"))
  (bind _nearactor (`self.IsNearGrabFunc` Sphere))
  (`/Engine/EditorBlueprintResources/StandardMacros.IsValid` _nearactor
    (:`Is Valid`
      (set `self.IsGrabbleAct` true)
      (bind _actor (message `/Game/Character/I__GrabAble.Grab` _nearactor MotionController))
      (set `self.AttachedActor` _actor)
      (`self.WhatActorRef`))))

(fn `IsNearGrabFunc`
  (params (Sphere :type "SphereComponent Object Reference"))
  (returns (NearActor :type "Actor Object Reference"))
  (for _array_element (`PrimitiveComponent.GetOverlappingActors` Sphere null)
    (if (`KismetSystemLibrary.DoesImplementInterface` _array_element "/Game/Character/I__GrabAble.I__GrabAble_C")
      (if (< (`KismetMathLibrary.VSize` (- (`self.K2_GetActorLocation` _array_element) (`SceneComponent.K2_GetComponentLocation` (`self.L_Sphere`)))) 300.0)
        (set `self.NearActor` _array_element))))
  (return (`self.NearActor`)))

(fn `ReleaseFunc`
  (params (MotionController :type "MotionControllerComponent Object Reference"))
  (bind _attachedactor (`self.AttachedActor`))
  (`/Engine/EditorBlueprintResources/StandardMacros.IsValid` _attachedactor
    (:`Is Valid`
      (if (== (`SceneComponent.GetAttachParent` (`self.K2_GetRootComponent` _attachedactor)) MotionController)
        (message `/Game/Character/I__GrabAble.Release` (`self.AttachedActor`)))
      (set `self.AttachedActor` null)
      (set `self.IsGrabbleAct` false)
      (set `self.NearActor` null))))

(fn `UserConstructionScript`)

(fn `WhatActorRef`
  (cast `/Game/UserInteractionActorBP/BP_Hammer` (`self.AttachedActor`))
  (set `self.IsHammer` true))